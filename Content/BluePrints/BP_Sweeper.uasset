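; BP_Sweeper is a first-person player Blueprint that uses its hands to carry objects and AI, or its tools to wipe graffiti.
; Use fires a short camera trace: items lerp to ItemArrow via timeline and attach, AI attach immediately with movement disabled, and tools apply their stats to graffiti.
; Dropping detaches the held actor and restores collision plus physics or AI movement.
; Holding Rotate enables input on the held item.
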(event `self.PutObject`
  (bind _interactobject (`self.InteractObject`))
  (bind _returnvalue (`self.GetComponentByClass` (`self.InteractObject`) "/Script/Engine.PrimitiveComponent"))
  (`parent.PutObject`)
  ;[1 1 1] Put Interactable Item
  (`/Engine/EditorBlueprintResources/StandardMacros.IsValid` (`self.InteractObject`) :!label _label
    (:`Is Valid`
      (`SceneComponent.K2_DetachFromComponent` (`self.ItemObject`) "KeepWorld" "KeepWorld" "KeepWorld" true)
      (`SceneComponent.K2_DetachFromComponent` (`Actor.RootComponent` (`self.InteractObject`)) "KeepWorld" "KeepWorld" "KeepWorld" true)
      (if (`self.ActorHasTag` (`self.InteractObject`) "AI")
        (bind _asaibase (cast `AIBase` (`self.InteractObject`)))
        (bind _asaicontroller_base (cast `AIControllerBase` (`self.GetController` _asaibase)))
        (`AIControllerBase.PutOut` _asaicontroller_base)
        (`ActorComponent.SetActive` (`self.GetComponentByClass` _interactobject "/Script/Engine.CharacterMovementComponent") true false)
        (`PrimitiveComponent.SetCollisionProfileName` (`self.GetComponentByClass` _interactobject "/Script/Engine.ShapeComponent") "Pawn" true)
        (else
          (`PrimitiveComponent.SetSimulatePhysics` _returnvalue true)
          (`PrimitiveComponent.SetCollisionProfileName` _returnvalue "InteractableActor" true)))
      (set `self.IsGrip` false)
      (set `self.InteractObject` null))))

(event `Inspect`
  (bind _firstpersoncameracomponent (`self.FirstPersonCameraComponent`))
  (bind _firstpersoncameracomponent_2 (`self.FirstPersonCameraComponent`))
  (bind _interactobject (`self.InteractObject`))
  (bind _interactobject_2 (`self.InteractObject`))
  (bind _returnvalue (`SceneComponent.K2_GetComponentLocation` _firstpersoncameracomponent_2))
  (bind _returnvalue_2 (`SceneComponent.K2_GetComponentLocation` _firstpersoncameracomponent))
  (bind _returnvalue_3 (`self.GetComponentByClass` _interactobject "/Script/Engine.ShapeComponent"))
  (if (`self.CanUseTool`) :!label _label_2
    (if (`|EnumEquality` (`self.CurrentTool`) "Hand")
      (if (`self.IsGrip`)
        (goto _label)
        (else
          ;[1 1 1] Check Interactable Object
          (bind (_outhit _returnvalue_4) (`KismetSystemLibrary.LineTraceSingle` _returnvalue (+ _returnvalue (* (`SceneComponent.GetForwardVector` _firstpersoncameracomponent_2) 250.0)) "TraceTypeQuery4"))
          (if _returnvalue_4
            (bind (_bblockinghit _binitialoverlap _time _distance _location _impactpoint _normal _impactnormal _physmat _hitactor) (`GameplayStatics.BreakHitResult` _outhit))
            (if (`self.ActorHasTag` _hitactor "Interactable")
              (bind _asbp_interactable_item_parent (cast `/Game/BluePrints/BP_InteractableItemParent` _hitactor))
              (if (`InteractableItemParent.IsInteractable` _asbp_interactable_item_parent)
                (set `self.IsGrip` true)
                (set `self.InteractObject` _hitactor)
                (`KismetSystemLibrary.Delay` 0.1)
                ;[1 1 1] Lerp Movement
                (set `self.StartLocation` (`SceneComponent.RelativeLocation` (`Actor.RootComponent` (`self.InteractObject`))))
                (set `self.EndLocation` (`SceneComponent.K2_GetComponentLocation` (`self.ItemArrow`)))
                (bind (_direction _item_track) (`Timeline|PickUpObject` :!via `PlayFromStart` :!label _label_3)
                  (:`Update`
                    (`/Engine/EditorBlueprintResources/StandardMacros.IsValid` _interactobject_2
                      (:`Is Valid`
                        (`SceneComponent.K2_SetRelativeLocation` (`Actor.RootComponent` _interactobject_2) (`KismetMathLibrary.VLerp` (`self.StartLocation`) (`self.EndLocation`) _item_track) false false)
                        (`self.K2_SetActorRelativeRotation` :`self` _interactobject_2))))
                  (:`Finished`
                    ;[1 1 1] PickUp Interactable Item
                    (bind _asbp_interactable_item_parent_2 (cast `/Game/BluePrints/BP_InteractableItemParent` (`self.InteractObject`)))
                    (`/Game/BluePrints/BP_InteractableItemParent.Start Inspect` _asbp_interactable_item_parent_2 self)
                    (bind _returnvalue_5 (`self.GetComponentByClass` _asbp_interactable_item_parent_2 "/Script/Engine.PrimitiveComponent"))
                    (`PrimitiveComponent.SetSimulatePhysics` _returnvalue_5 false)
                    (`PrimitiveComponent.SetCollisionProfileName` _returnvalue_5 "GripActor" true)
                    (`self.K2_AttachToComponent` _asbp_interactable_item_parent_2 (`self.ItemArrow`) "None" "SnapToTarget" "KeepWorld" "KeepWorld" true))))
              (else
                ;[1 1 1] Check AI
                (if (`self.ActorHasTag` _hitactor "AI")
                  (bind _asaibase (cast `AIBase` _hitactor))
                  (if (`AIBase.IsInteractable` _asaibase)
                    (set `self.IsGrip` true)
                    (set `self.InteractObject` _asaibase)
                    ;[1 1 1] PickUp AI
                    (bind _asaicontroller_base (cast `AIControllerBase` (`self.GetController` _asaibase)))
                    (`AIControllerBase.PutOn` _asaicontroller_base)
                    (`ActorComponent.SetActive` (`self.GetComponentByClass` _interactobject "/Script/Engine.CharacterMovementComponent") false false)
                    (`PrimitiveComponent.SetSimulatePhysics` _returnvalue_3 false)
                    (`PrimitiveComponent.SetCollisionProfileName` _returnvalue_3 "GripActor" true)
                    (`self.K2_AttachToComponent` _interactobject (`self.ItemArrow`) "None" "SnapToTarget" "SnapToTarget" "KeepWorld" true)
                    (bind _asaibase_2 (cast `AIBase` (`self.InteractObject`)))
                    (set `AIBase.IsGrounded` false _asaibase_2))))))))
      (else
        ;[1 1 1] Check Graffiti
        (bind (_outhit_2 _returnvalue_6) (`KismetSystemLibrary.LineTraceSingle` _returnvalue_2 (+ _returnvalue_2 (* (`SceneComponent.GetForwardVector` _firstpersoncameracomponent) 250.0)) "TraceTypeQuery4" false (`self.Actors to Ignore`) "ForDuration"))
        (if _returnvalue_6
          (bind (_bblockinghit_2 _binitialoverlap_2 _time_2 _distance_2 _location_2 _impactpoint_2 _normal_2 _impactnormal_2 _physmat_2 _hitactor_2) (`GameplayStatics.BreakHitResult` _outhit_2))
          (if (`self.ActorHasTag` _hitactor_2 "Interactable")
            ;[1 1 1] Wipe Graffiti
            (bind _asbp_graffiti_obs_base (cast `/Game/BluePrints/GraffitiObstacle/BP_GraffitiObsBase` _hitactor_2))
            (`GraffitiObstacle.WipeObstacle` _asbp_graffiti_obs_base (`self.CurrentTool`) (`.RemoveDamage` (break `ToolStat` (`|GetArrayItem` (`self.ToolStats`) (`KismetMathLibrary.Conv_ByteToInt` (`self.CurrentTool`))))))))))))

(event `MissingItem`
  ;[1 1 1] Lerp Movement
  (goto _label_3 :!via `Stop`))

(event `InputAction|Use`
  (params (Key :type "Key Structure"))
  (:`Pressed`
    (goto _label_2)))

(event `InputAction|Rotate`
  (params (Key :type "Key Structure"))
  ;[1 1 1] Interactable Object Rotate Event
  (:`Pressed`
    (`self.SetEnableInputInteractableObject` true))
  (:`Released`
    (`self.SetEnableInputInteractableObject` false)))

(fn `SetEnableInputInteractableObject`
  (params (IsEnable :type Boolean))
  (bind _interactobject (`self.InteractObject`))
  (`/Engine/EditorBlueprintResources/StandardMacros.IsValid` _interactobject
    (:`Is Valid`
      (bind _asbp_interactable_item_parent (cast `/Game/BluePrints/BP_InteractableItemParent` _interactobject))
      (if (`self.IsGrip`)
        (`/Game/BluePrints/BP_InteractableItemParent.SetEnableInput` _asbp_interactable_item_parent IsEnable)))))

(fn `UserConstructionScript`)
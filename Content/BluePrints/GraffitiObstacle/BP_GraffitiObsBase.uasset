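; Base Blueprint for a wipeable graffiti obstacle that ties its creation and cleaning to the game's cleaning progress.
; Creation runs the parent logic only if total progress stays positive after the penalty, then deducts ProgressValue from Remove progress, falling back to Organize.
; Completing a wipe calls the parent and adds the value back in the same order, respecting each category's cap.
; SetMaterial and the construction script are empty.
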(event `SetMaterial`
  (params (count :type Integer)))

(event `self.CreateGraffitiObstacle`
  (bind _returnvalue (subsystem `CleaningManager`))
  (bind _returnvalue_2 (subsystem `CleaningManager`))
  (bind _returnvalue_3 (* -1 (`self.ProgressValue`)))
  (bind _returnvalue_4 (* -1 (`self.ProgressValue`)))
  (`/Engine/EditorBlueprintResources/StandardMacros.IsValid` _returnvalue
    (:`Is Valid`
      (if (> (+ (`CleaningManager.TotalProgress` _returnvalue) (* -1 (`self.ProgressValue`))) 0.0)
        (`parent.CreateGraffitiObstacle`)
        (`/Engine/EditorBlueprintResources/StandardMacros.IsValid` _returnvalue_2
          (:`Is Valid`
            (if (>= (+ (`CleaningManager.RemoveProgress` _returnvalue_2) _returnvalue_4) 0.0)
              (`CleaningManager.SetProgress` _returnvalue_2 "Remove" _returnvalue_4)
              (elif (>= (+ (`CleaningManager.OrganizeProgress` _returnvalue_2) _returnvalue_3) 0.0)
                (`CleaningManager.SetProgress` _returnvalue_2 "Organize" _returnvalue_3)))))))))

(event `self.CompleteWipe`
  (bind _returnvalue (subsystem `CleaningManager`))
  (bind _progressvalue (`self.ProgressValue`))
  (bind _progressvalue_2 (`self.ProgressValue`))
  (`parent.CompleteWipe`)
  (`/Engine/EditorBlueprintResources/StandardMacros.IsValid` _returnvalue
    (:`Is Valid`
      (if (<= (+ (`CleaningManager.RemoveProgress` _returnvalue) _progressvalue_2) 50.0)
        (`CleaningManager.SetProgress` _returnvalue "Remove" _progressvalue_2)
        (elif (<= (+ (`CleaningManager.OrganizeProgress` _returnvalue) _progressvalue) 50.0)
          (`CleaningManager.SetProgress` _returnvalue "Organize" _progressvalue))))))

(fn `UserConstructionScript`)
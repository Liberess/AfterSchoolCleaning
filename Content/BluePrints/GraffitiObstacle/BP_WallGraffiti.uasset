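; BP_WallGraffiti is a wall graffiti obstacle that shows a randomly chosen graffiti material with count-driven opacity.
; The construction script calls its parent, then creates a dynamic material instance on the mesh from a random entry in the SourceMaterial array.
; The SetMaterial event lowers that instance's Opacity in thirds as Count rises, but sets it back to fully opaque once Count reaches three or more.
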(event `self.SetMaterial`
  (params (count :type Integer))
  (bind _returnvalue (* count (/ 1.0 3.0)))
  (if (>= _returnvalue 1.0)
    (`MaterialInstanceDynamic.SetScalarParameterValue` (`self.MaterialInstance`) "Opacity" 1.0)
    (else
      (`MaterialInstanceDynamic.SetScalarParameterValue` (`self.MaterialInstance`) "Opacity" (- 1.0 _returnvalue)))))

(fn `UserConstructionScript`
  (`parent.UserConstructionScript`)
  (bind _returnvalue (`PrimitiveComponent.CreateDynamicMaterialInstance` (`self.mesh`) 0 (`|GetArrayItem` (`self.Source Material`) (`KismetMathLibrary.RandomInteger` (`KismetArrayLibrary.Array_Length` (`self.Source Material`)))) "None"))
  (set `self.MaterialInstance` _returnvalue))
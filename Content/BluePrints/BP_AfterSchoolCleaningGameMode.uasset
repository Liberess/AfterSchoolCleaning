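; Game mode Blueprint for the After School Cleaning game that shows tool buff countdowns on the in-game UI.
; SetBuffUI casts the current widget to UI_InGame and picks the wall or floor buff by obstacle type.
; Each has its own timeline, with play rate scaled inversely by Duration, that restarts and lerps the widget's buff value from full to zero.
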(event `self.SetBuffUI`
  (params (ObsType :type "EObstacleType Enum" :default "WallObs") (Duration :type "Float (single-precision)"))
  (bind _currentwidget (`self.CurrentWidget`))
  (bind _wallbufftimeline (`self.WallBuffTimeline`))
  (bind _floorbufftimeline (`self.FloorBuffTimeline`))
  (bind _returnvalue (`TimelineComponent.GetTimelineLength` _wallbufftimeline))
  (bind _returnvalue_2 (`TimelineComponent.GetTimelineLength` _floorbufftimeline))
  (`/Engine/EditorBlueprintResources/StandardMacros.IsValid` _currentwidget
    (:`Is Valid`
      (bind _asui_in_game (cast `/Game/UI/UI_InGame` _currentwidget))
      (switch `EObstacleType` ObsType
        (:`WallObs`
          (`/Game/UI/UI_InGame.WallToolBuff` _asui_in_game 1.0)
          (`TimelineComponent.SetPlayRate` _wallbufftimeline (/ _returnvalue (* _returnvalue Duration)))
          (bind (_direction _time) (`Timeline|WallBuffTimeline` :!via `PlayFromStart`)
            (:`Update`
              (`/Game/UI/UI_InGame.WallToolBuff` _asui_in_game (`KismetMathLibrary.Lerp` 1.0 0.0 _time)))))
        (:`FloorObs`
          (`/Game/UI/UI_InGame.FloorToolBuff` _asui_in_game 1.0)
          (`TimelineComponent.SetPlayRate` _floorbufftimeline (/ _returnvalue_2 (* _returnvalue_2 Duration)))
          (bind (_direction_2 _time_2) (`Timeline|FloorBuffTimeline` :!via `PlayFromStart`)
            (:`Update`
              (`/Game/UI/UI_InGame.FloorToolBuff` _asui_in_game (`KismetMathLibrary.Lerp` 1.0 0.0 _time_2)))))))))

(fn `UserConstructionScript`)
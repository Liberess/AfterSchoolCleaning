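; Parent Blueprint for interactable items that the player can inspect and rotate.
; StartInspect stores the inspector, clears IsGrounded and enables input on the item.
; While right mouse is held, mouse X and Y roll and pitch the item mesh through combined rotators; otherwise the axis events disable the item's input.
; Pressing Use calls Inspect on the inspecting BP_Sweeper.
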(event `Start Inspect`
  (params (Inspector :type "Pawn Object Reference"))
  ;[1 1 1] Start and Stop Inspect
  (set `self.Inspector` Inspector)
  (`self.SetEnableInput` true)
  (set `self.IsGrounded` false))

(event `InputAction|Use`
  (params (Key :type "Key Structure"))
  ;[1 1 1] Start and Stop Inspect
  (:`Pressed`
    (bind _asbp_sweeper (cast `/Game/BluePrints/BP_Sweeper` (stale `Start Inspect` Inspector)))
    (`/Game/BluePrints/BP_Sweeper.Inspect` _asbp_sweeper)))

(event `InputAxisKey|MouseX`
  (params (AxisValue :type "Float (single-precision)"))
  ;[1 1 1] Rotate
  (if (`PlayerController.IsInputKeyDown` (`GameplayStatics.GetPlayerController` 0) "RightMouseButton")
    (`self.SetEnableInput` true)
    (`SceneComponent.K2_SetRelativeRotation` (`self.ItemMesh`) (`KismetMathLibrary.ComposeRotators` (`SceneComponent.RelativeRotation` (`self.ItemMesh`)) (`KismetMathLibrary.MakeRotator` (* AxisValue -1.0))) false false)
    (else
      (`self.SetEnableInput` false))))

(event `InputAxisKey|MouseY`
  (params (AxisValue :type "Float (single-precision)"))
  ;[1 1 1] Rotate
  (if (`PlayerController.IsInputKeyDown` (`GameplayStatics.GetPlayerController` 0) "RightMouseButton")
    (`self.SetEnableInput` true)
    (`SceneComponent.K2_SetRelativeRotation` (`self.ItemMesh`) (`KismetMathLibrary.ComposeRotators` (`SceneComponent.RelativeRotation` (`self.ItemMesh`)) (`KismetMathLibrary.MakeRotator` 0.0 (* AxisValue -1.0))) false false)
    (else
      (`self.SetEnableInput` false))))

(fn `SetEnableInput`
  (params (IsEnable :type Boolean))
  (bind _returnvalue (`GameplayStatics.GetPlayerController` 0))
  (bind _output_get (set `self.IsRotate` IsEnable))
  (if _output_get
    (`self.EnableInput` _returnvalue)
    (else
      (`self.DisableInput` _returnvalue))))

(fn `UserConstructionScript`)